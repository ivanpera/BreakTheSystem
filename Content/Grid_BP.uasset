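; Grid Blueprint that spawns chains on demand, with unfinished logic for stepping its grid elements.
; Tick treats the Asd flag as a one-shot trigger, clearing it and calling SpawnChain.
; A timed update that would move every valid Grid element by one in Y and then call ApplyMoves is disconnected.
; The remaining-time check on Tick leads nowhere, so this graph never runs that movement.
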(event EventTick
  (params (DeltaSeconds :type Float%20%28single-precision%29))
  (if (Variables|Default|Getasd)
    (Variables|Default|Setasd false)
    (Class|Grid|SpawnChain)
    (elif (<= (Variables|Default|GetUpdateRemainingTime) 0.0)
      _)))

(fn ConstructionScript)