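; Player controller for a grid-based falling-piece game that forwards rotate, sideways and downward input to the Grid.
; BeginPlay takes the Grid from the first GridContainer actor in the level, and rotation is sent to it immediately on press.
; Held move keys set flags that Tick repeats on a countdown timer, reset on release.
; Releasing one sideways key reverts movement to the opposite key if still held.
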(event EventTick
  (params (DeltaSeconds :type Float%20%28single-precision%29))
  (if (<= (Variables|Default|GetCurrInputThresholdTime) 0.0)
    (if (or (Variables|Default|GetMoveLeft) (Variables|Default|GetMoveRight))
      (Class|Grid|OnMove (Variables|Default|GetGrid) (Variables|Default|GetMovement)))
    (if (Variables|Default|GetMoveDown)
      (Class|Grid|OnForceDown (Variables|Default|GetGrid)))
    (Variables|Default|SetCurrInputThresholdTime (Variables|Default|GetIntputThresholdTime))
    (else
      (Variables|Default|SetCurrInputThresholdTime (- (Variables|Default|GetCurrInputThresholdTime) DeltaSeconds)))))

(event EventBeginPlay
  (bind _outactors (Actor|GetAllActorsOfClass "/Game/GridContainer.GridContainer_C"))
  (Variables|Default|SetGrid (Variables|/Game/GridContainer.GridContainer_C|GetGrid (Utilities|Array|Get(acopy) _outactors))))

(event Input|ActionEvents|InputActionRotate
  (params (Key :type Key%20Structure :default "None"))
  (:Pressed
    (Class|Grid|OnRotate (Variables|Default|GetGrid))))

(event Input|ActionEvents|InputActionMoveLeft
  (params (Key :type Key%20Structure :default "None"))
  (:Pressed
    (Variables|Default|SetMovement "(X=-1.000000,Y=0.000000)")
    (Variables|Default|SetMoveLeft true))
  (:Released
    (Variables|Default|SetMoveLeft false)
    (Variables|Default|SetCurrInputThresholdTime 0.0)
    (if (Variables|Default|GetMoveRight)
      (Variables|Default|SetMovement "(X=1.000000,Y=0.000000)"))))

(event Input|ActionEvents|InputActionMoveRight
  (params (Key :type Key%20Structure :default "None"))
  (:Pressed
    (Variables|Default|SetMovement "(X=1.000000,Y=0.000000)")
    (Variables|Default|SetMoveRight true))
  (:Released
    (Variables|Default|SetMoveRight false)
    (Variables|Default|SetCurrInputThresholdTime 0.0)
    (if (Variables|Default|GetMoveLeft)
      (Variables|Default|SetMovement "(X=-1.000000,Y=0.000000)"))))

(event Input|ActionEvents|InputActionMoveDown
  (params (Key :type Key%20Structure :default "None"))
  (:Pressed
    (Variables|Default|SetMoveDown true))
  (:Released
    (Variables|Default|SetMoveDown false)
    (Variables|Default|SetCurrInputThresholdTime 0.0)))

(fn ConstructionScript)